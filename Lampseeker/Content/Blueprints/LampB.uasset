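; LampB is an interactable lamp actor that the player can switch on while standing near it.
; Its Box trigger enables input from player 0's controller on overlap and disables it when the overlap ends.
; Pressing L makes the SpotLight and PointLight visible, with no toggle back off, then sets Lightdim on the player's Pawn_Blueprint to a fixed value.
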(event OnComponentBeginOverlap(Box)
  (params (OverlappedComponent :type Primitive%20Component%20Object%20Reference) (OtherActor :type Actor%20Object%20Reference) (OtherComp :type Primitive%20Component%20Object%20Reference) (OtherBodyIndex :type Integer) (bFromSweep :type Boolean) (SweepResult :type Hit%20Result%20Structure%20%28by%20ref%29))
  (Input|EnableInput (Game|GetPlayerController 0)))

(event OnComponentEndOverlap(Box)
  (params (OverlappedComponent :type Primitive%20Component%20Object%20Reference) (OtherActor :type Actor%20Object%20Reference) (OtherComp :type Primitive%20Component%20Object%20Reference) (OtherBodyIndex :type Integer))
  (Input|DisableInput (Game|GetPlayerController 0)))

(event EventBeginPlay)

(event Collision|EventActorBeginOverlap
  (params (OtherActor :type Actor%20Object%20Reference)))

(event EventTick
  (params (DeltaSeconds :type Float%20%28single-precision%29)))

(event Input|KeyboardEvents|L
  (params (Key :type Key%20Structure))
  (:Pressed
    (Rendering|SetVisibility (Variables|Default|GetSpotLight) true false)
    (bind _aspawn_blueprint (Utilities|Casting|CastToPawn_Blueprint (Game|Player|GetPlayerPawn 0)))
    (Variables|/Game/TopDownBP/Blueprints/Pawn_Blueprint.Pawn_Blueprint_C|Setlightdim _aspawn_blueprint 7.2e+04)))

(fn ConstructionScript)